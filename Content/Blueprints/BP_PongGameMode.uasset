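; Game mode for local multiplayer Pong that runs player setup, countdowns, score display and the game-over screen.
; On BeginPlay it creates a local player per PlayerStart with Enhanced Input and a possessed paddle, recolouring the first player's.
; Countdown macros animate a widget through chained one-second delays before each LaunchBall call.
; ShowPointScored hides the score during that countdown, while ShowGameOver displays the winner.
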(event EventBeginPlay
  (|InitPlayers)
  (Audio|PlaySound2D "/Game/Retro_8Bit_Sounds/Music/Cues/retro__musical_stinger_02_Cue.retro__musical_stinger_02_Cue" 1.0 1.0 0.0 0 0)
  (|CountdownAnim_2_2
    (:Completed
      (bind _returnvalue (UserInterface|CreateWidget "/Game/UI/ScoreWidget.ScoreWidget_C"))
      (bind _output_get (Variables|Default|SetScoreDisplay _returnvalue))
      (UserInterface|Viewport|AddtoPlayerScreen _output_get)
      (Class|PongGameModeBase|LaunchBall))))

(event EventShowPointScored
  (params (scoringPlayer :type Integer))
  (Widget|RemovefromParent (Variables|Default|GetScoreDisplay))
  (Audio|PlaySound2D "/Game/Retro_8Bit_Sounds/Retro_Orginal/Cues/retro_beeps_collect_item_01_Cue.retro_beeps_collect_item_01_Cue" 1.0 1.0 0.0 0 0)
  (|CountdownAnim scoringPlayer
    (:Completed
      (Audio|PlaySound2D "/Game/Retro_8Bit_Sounds/Retro_Orginal/Cues/retro_synth_beeps_08_Cue.retro_synth_beeps_08_Cue" 1.0 1.0 0.0 0 0)
      (Class|PongGameModeBase|LaunchBall)
      (UserInterface|Viewport|AddtoPlayerScreen (Variables|Default|GetScoreDisplay)))))

(event EventShowGameOver
  (params (scoringPlayer :type Integer))
  (Widget|RemovefromParent (Variables|Default|GetScoreDisplay))
  (bind _returnvalue (UserInterface|CreateWidget "/Game/UI/GameOver.GameOver_C"))
  (Variables|/Game/UI/GameOver.GameOver_C|SetDisplayText _returnvalue (Utilities|Text|ToText(String) (Utilities|String|Append "PLAYER " (Utilities|String|ToString(Integer) scoringPlayer) " WINS")))
  (UserInterface|Viewport|AddtoPlayerScreen _returnvalue)
  (Audio|PlaySound2D "/Game/Retro_8Bit_Sounds/Music/Cues/retro__musical_stinger_03_Cue.retro__musical_stinger_03_Cue" 1.0 1.0 0.0 0 0))

(fn ConstructionScript)